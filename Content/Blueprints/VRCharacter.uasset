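; VR player character with motion-controller grabbing, smooth locomotion and stick turning.
; Grab inputs check each hand's collision for overlapping actors implementing GrippableInterface, send them GrabMessage with that motion controller, and store one per hand to receive ReleaseMessage on release.
; The left stick moves along the camera's forward and right vectors, while the right stick's X axis applies frame-time-scaled yaw.
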(event Input|ActionEvents|InputActionGrabRight
  (params (Key :type Key%20Structure :default "None"))
  ;[1 1 1] Grip
  (:Pressed
    (for _array_element (Collision|GetOverlappingActors (Variables|Default|GetCollisionRight) 0 :!class /Script/Engine.PrimitiveComponent)
      (if (Utilities|DoesObjectImplementInterface _array_element "/Game/Interfaces/GrippableInterface.GrippableInterface_C")
        (Class|GrippableInterface|Grab(Message) _array_element (Variables|Default|GetMotionControllerRight))
        (Variables|Default|SetGrab%20Right%20Actor _array_element))))
  (:Released
    (Utilities|IsValid (Variables|Default|GetGrab%20Right%20Actor)
      (:Is%20Valid
        (Class|GrippableInterface|Release(Message) (Variables|Default|GetGrab%20Right%20Actor))))))

(event Input|ActionEvents|InputActionGrabLeft
  (params (Key :type Key%20Structure :default "None"))
  ;[1 1 1] Grip
  (:Pressed
    (for _array_element (Collision|GetOverlappingActors (Variables|Default|GetCollisionLeft) 0 :!class /Script/Engine.PrimitiveComponent)
      (if (Utilities|DoesObjectImplementInterface _array_element "/Game/Interfaces/GrippableInterface.GrippableInterface_C")
        (Class|GrippableInterface|Grab(Message) _array_element (Variables|Default|GetMotionControllerLeft))
        (Variables|Default|SetGrabLeftActor _array_element))))
  (:Released
    (Utilities|IsValid (Variables|Default|GetGrabLeftActor)
      (:Is%20Valid
        (Class|GrippableInterface|Release(Message) (Variables|Default|GetGrabLeftActor))))))

(event Input|AxisEvents|InputAxisMovementAxisRight_X
  (params (AxisValue :type Float%20%28single-precision%29))
  ;[1 1 1] Player Look Rotation
  (Pawn|Input|AddControllerYawInput (* AxisValue (* (Utilities|Time|GetWorldDeltaSeconds) (Variables|Default|GetRotation%20Speed)))))

(event Input|AxisEvents|InputAxisMovementAxisRight_Y
  (params (AxisValue :type Float%20%28single-precision%29)))

(event Input|AxisEvents|InputAxisMovementAxisLeft_X
  (params (AxisValue :type Float%20%28single-precision%29))
  ;[1 1 1] Player Movement
  (Pawn|Input|AddMovementInput (Math|Vector|GetRightVector (Variables|Camera|GetCamera)) (* AxisValue (Variables|Default|GetMovement%20Speed)) false))

(event Input|AxisEvents|InputAxisMovementAxisLeft_Y
  (params (AxisValue :type Float%20%28single-precision%29))
  ;[1 1 1] Player Movement
  (Pawn|Input|AddMovementInput (Math|Vector|GetForwardVector (Variables|Camera|GetCamera)) (* AxisValue (Variables|Default|GetMovement%20Speed)) false))

(fn ConstructionScript)